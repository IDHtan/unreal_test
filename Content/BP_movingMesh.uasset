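; BP_movingMesh is an actor that moves its static mesh from a start location toward an end location.
; BeginPlay snaps the mesh to the start, stores the offset to the end and sets the Movement timeline's play rate to Speed divided by distance.
; Tick calls Play every frame, and the timeline's update places the mesh along that offset using its T track, without sweeping.
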(event EventBeginPlay
  (Transformation|SetWorldLocation (Variables|Default|GetStaticMesh) (Variables|Default|GetstartLocation) false false)
  (Variables|Default|SetmoveDirection (- (Variables|Default|GetendLocation) (Variables|Default|GetstartLocation)))
  (bind _output_get (Variables|Default|SetplayRate (/ (Variables|Default|Getspeed) (Math|Vector|Distance(Vector) (Variables|Default|GetstartLocation) (Variables|Default|GetendLocation)))))
  (Components|Timeline|SetPlayRate (Variables|Default|Getmovement) _output_get))

(event EventTick
  (params (DeltaSeconds :type Float%20%28single-precision%29))
  (bind _t (Timeline|movement Play)
    (:Update
      (Transformation|SetWorldLocation (Variables|Default|GetStaticMesh) (+ (* _t (Variables|Default|GetmoveDirection)) (Variables|Default|GetstartLocation)) false false))))

(fn ConstructionScript)