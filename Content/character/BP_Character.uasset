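; BP_Character is a player character Blueprint that provides basic movement and look control through Enhanced Input.
; On BeginPlay it adds the IMC_Input mapping context to the first player controller's input subsystem.
; IA_Move2 drives movement along the actor's own axes, with X as forward and Y as right.
; IA_Look2 feeds X and Y into controller yaw and pitch.
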(event Input|EnhancedActionEvents|EnhancedInputActionIA_Move2
  (params (ActionValue :type Vector%202D%20Structure) (ElapsedSeconds :type Float%20%28double-precision%29) (TriggeredSeconds :type Float%20%28double-precision%29) (InputAction :type Input%20Action%20Object%20Reference :default "/Game/character/IA_Move2.IA_Move2"))
  (bind (_x _y) (Math|Vector2D|BreakVector2D ActionValue))
  (Pawn|Input|AddMovementInput (Transformation|GetActorForwardVector) _x false)
  (Pawn|Input|AddMovementInput (Transformation|GetActorRightVector) _y false))

(event Input|EnhancedActionEvents|EnhancedInputActionIA_Look2
  (params (ActionValue :type Vector%202D%20Structure) (ElapsedSeconds :type Float%20%28double-precision%29) (TriggeredSeconds :type Float%20%28double-precision%29) (InputAction :type Input%20Action%20Object%20Reference :default "/Game/character/IA_Look2.IA_Look2"))
  (bind (_x _y) (Math|Vector2D|BreakVector2D ActionValue))
  (:Triggered
    (Pawn|Input|AddControllerYawInput _x)
    (Pawn|Input|AddControllerPitchInput _y)))

(event EventBeginPlay
  (Input|AddMappingContext (PlayerController|LocalPlayerSubsystems|GetEnhancedInputLocalPlayerSubsystem (Game|GetPlayerController 0)) "/Game/character/IMC_Input.IMC_Input" 0 "(bIgnoreAllPressedKeysUntilRelease=True,bForceImmediately=False,bNotifyUserSettings=False)"))

(fn ConstructionScript)